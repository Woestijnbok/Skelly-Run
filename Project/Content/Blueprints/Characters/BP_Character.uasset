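; Base 2D flipbook character with movement, jumping, melee attacks and death, with BP_Player getting special death handling.
; A state enum selects each flipbook, while Tick drives transitions from sprite playback and velocity.
; Attacks are interval-gated and damage the character found by a forward line trace on a set animation frame.
; Health component events trigger sounds, timed hit flicker that blocks attacking, and death, ending in HUD notification and pause or destruction.
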(event `self.End Falling`
  (bind _returnvalue_x (`KismetMathLibrary.BreakVector` (`self.GetVelocity`)))
  ;[1 1 1] Event end falling, called once when we reach the ground again
  (set `self.On Ground` true)
  (if (== _returnvalue_x 0.0)
    (`self.Set Character State` "NewEnumerator0" true)))

(event `self.ReceiveTick`
  (params (DeltaSeconds :type "Float (single-precision)"))
  ;[1 1 1] Even Tick
  (`self.Update Character State` DeltaSeconds))

(event `self.ReceiveBeginPlay`
  ;[1 1 1] Event BeginPlay
  (`self.Set Character State` "NewEnumerator3"))

(event `self.End Attack`
  ;[1 1 1] Event end attack, called once when attack animation finishes
  (`self.Set Character State` "NewEnumerator0" true))

(event `self.Moving`
  (params (`Action Value` :type "Float (double-precision)"))
  ;[1 1 1] Moving event, called when character is moving vertically
  (if (and (`self.Is Not Attacking`) (`self.Is Alive`))
    (`self.Flip Sprite` (> `Action Value` 0.0))
    (`self.AddMovementInput` (`self.GetActorForwardVector`))
    (if (`self.On Ground`)
      (`self.Set Character State` "NewEnumerator1" true))))

(event `self.Start Jump`
  ;[1 1 1] Event start jump, called once when starting to jump
  (if (and (and (`self.Is Not Attacking`) (`self.On Ground`)) (`self.Is Alive`))
    (`self.Jump`)
    (`self.Set Character State` "NewEnumerator2")
    (set `self.On Ground` false)))

(event `self.Try Attack`
  ;[1 1 1] Event attack, called when starting to attack
  (if (and (and (`self.Is Not Attacking`) (and (not (`KismetSystemLibrary.K2_IsTimerActive` null "Toggle Sprite Visibiltiy")) (and (`self.On Ground`) (>= (`self.Attack Interval Timer`) (`self.Attack Interval`))))) (`self.Is Alive`))
    (`self.Set Character State` "NewEnumerator4")))

(event `self.Peak Jump`
  ;[1 1 1] Event peak jump, called once when reached apex point in jump arc
  (`self.Set Character State` "NewEnumerator3"))

(event `self.Character Health (HealthComponent).OnDamage`
  (params (DamageAmount :type "Float (single-precision)"))
  ;[1 1 1] On Damage event
  (`KismetSystemLibrary.K2_ClearTimer` null "Toggle Sprite Visibiltiy")
  (`KismetSystemLibrary.K2_SetTimer` null "Toggle Sprite Visibiltiy" 0.2 true)
  (`GameplayStatics.PlaySound2D` (`self.Hit Sound`) 1.0 1.0 0.0 null null))

(event `self.End Moving`
  ;[1 1 1] Event stopt moving, called once when character stopt moving horizontally
  (if (and (and (`self.Is Not Attacking`) (`self.On Ground`)) (`self.Is Alive`))
    (`self.Set Character State` "NewEnumerator0" true)))

(event `self.Character Health (HealthComponent).OnDeath`
  ;[1 1 1] On Death event
  (`self.Set Character State` "NewEnumerator5")
  (`GameplayStatics.PlaySound2D` (`self.Death Sound`) 1.0 1.0 0.0 null null)
  (`PrimitiveComponent.SetCollisionEnabled` (`self.CapsuleComponent`) "NoCollision"))

(fn `Flip Sprite`
  (params (`Facing Right` :type Boolean))
  (if `Facing Right`
    (`SceneComponent.K2_SetWorldRotation` :`self` (`self.CapsuleComponent`))
    (else
      (`SceneComponent.K2_SetWorldRotation` (`self.CapsuleComponent`) (struct :`Yaw` 180.0) false false))))

(fn `Get Character In Front`
  (returns (Valid :type Boolean) (Character :type "/Game/Blueprints/Characters/BP_Character Object Reference"))
  (bind (_returnvalue_x _returnvalue_y _returnvalue_z) (`KismetMathLibrary.BreakVector` (`self.K2_GetActorLocation`)))
  (bind _returnvalue (`KismetMathLibrary.MakeVector` _returnvalue_x _returnvalue_y (+ _returnvalue_z (`self.Trace Height Offset`))))
  ;[1 1 1] Line trace for pawn objects
  (bind (_outhit _returnvalue_2) (`KismetSystemLibrary.LineTraceSingleForObjects` _returnvalue (+ _returnvalue (* (`self.GetActorForwardVector`) (`self.Attack Range`))) (`self.Objects To Trace`)))
  ;[1 1 1] Check if there was a hit, ifso also check if it was a character
  (if _returnvalue_2
    (bind _asbp_character (cast `/Game/Blueprints/Characters/BP_Character` (`.HitActor` (`GameplayStatics.BreakHitResult` _outhit)))
      (:`then`
        (return true _asbp_character))
      (:`CastFailed`
        _)))
  (return false null))

(fn `Is Alive`
  (returns (`Is ALive` :type Boolean))
  (return (not (`HealthComponent.IsDead` (`self.Character Health (HealthComponent)`)))))

(fn `Is Not Attacking`
  (returns (`Is Not Attacking` :type Boolean))
  (return (`|EnumInequality` (`self.Character State`) "NewEnumerator4")))

(fn `Set Character State`
  (params (`New State` :type "/Game/Enumerations/CharacterState Enum" :default "NewEnumerator0") (`Sprite Looping` :type Boolean))
  (if (`|EnumInequality` `New State` (`self.Character State`))
    (switch `/Game/Enumerations/CharacterState` `New State`
      (:`NewEnumerator0`
        (`PaperFlipbookComponent.SetFlipbook` (`self.Sprite`) (`self.Flipbook Idle`)))
      (:`NewEnumerator1`
        (`PaperFlipbookComponent.SetFlipbook` (`self.Sprite`) (`self.Flipbook Walk`)))
      (:`NewEnumerator2`
        (`PaperFlipbookComponent.SetFlipbook` (`self.Sprite`) (`self.Flipbook Jump`)))
      (:`NewEnumerator3`
        (`PaperFlipbookComponent.SetFlipbook` (`self.Sprite`) (`self.Flipbook Falling`)))
      (:`NewEnumerator4`
        (`PaperFlipbookComponent.SetFlipbook` (`self.Sprite`) (`self.Flipbook Attack`)))
      (:`NewEnumerator5`
        (`PaperFlipbookComponent.SetFlipbook` (`self.Sprite`) (`self.Flipbook Dying`))))
    (`PaperFlipbookComponent.SetLooping` (`self.Sprite`) `Sprite Looping`)
    (`PaperFlipbookComponent.PlayFromStart` (`self.Sprite`))
    (bind _output_get (set `self.Character State` `New State`))
    (`KismetSystemLibrary.LogString` (`|GetEnumeratorNameAsString` _output_get))))

(fn `Toggle Sprite Visibiltiy`
  (`SceneComponent.ToggleVisibility` (`self.Sprite`) true))

(fn `Update Character State`
  (params (`Delta Seconds` :type "Float (double-precision)"))
  (locals (Delta :type "Float (double-precision)"))
  (bind (_returnvalue_x _returnvalue_y _returnvalue_z) (`KismetMathLibrary.BreakVector` (`self.GetVelocity`)))
  (bind (_returnvalue_x_2 _returnvalue_y_2 _returnvalue_z_2) (`KismetMathLibrary.BreakVector` (`self.GetVelocity`)))
  (bind (_valid _character) (`self.Get Character In Front`))
  (set `local.Delta` `Delta Seconds`)
  ;[1 1 1] Check if death animation ended
  (if (and (not (`PaperFlipbookComponent.IsPlaying` (`self.Sprite`))) (`|EnumEquality` (`self.Character State`) "NewEnumerator5"))
    (cast `/Game/Blueprints/Characters/BP_Player` self
      (:`then`
        (bind _asbp_hud (cast `/Game/Blueprints/HUD/BP_HUD` (`PlayerController.GetHUD` (`GameplayStatics.GetPlayerController` 0))))
        (`/Game/Blueprints/HUD/BP_HUD.Player Death` _asbp_hud)
        (`GameplayStatics.SetGamePaused` true))
      (:`CastFailed`
        (`self.K2_DestroyActor`)))
    (else
      ;[1 1 1] Update Attack Interval Timer
      (if (and (`|EnumInequality` (`self.Character State`) "NewEnumerator4") (< (`self.Attack Interval Timer`) (`self.Attack Interval`)))
        (set `self.Attack Interval Timer` (+ (`local.Delta`) (`self.Attack Interval Timer`))))
      ;[1 1 1] Update flicker timer
      (if (`KismetSystemLibrary.K2_IsTimerActive` null "Toggle Sprite Visibiltiy")
        (bind _output_get (set `self.Flicker Timer` (+ (`self.Flicker Timer`) (`local.Delta`))))
        (if (>= _output_get (`self.Flicker Duration`))
          (`KismetSystemLibrary.K2_ClearTimer` null "Toggle Sprite Visibiltiy")
          (set `self.Flicker Timer` 0.0)
          (`SceneComponent.SetVisibility` (`self.Sprite`) true true)))
      ;[1 1 1] Check if we need to do damage
      ;;[1 1 1] Deal damage to the character in front if there are any
      (if (and (and (`|EnumEquality` (`self.Character State`) "NewEnumerator4") (== (`PaperFlipbookComponent.GetPlaybackPositionInFrames` (`self.Sprite`)) (`self.Damage Frame`))) (not (`self.Attacked This Frame`)))
        (if _valid
          (`HealthComponent.DoDamage` (`/Game/Blueprints/Characters/BP_Character.Character Health (HealthComponent)` _character) (`self.Damage Amount`)))
        (set `self.Attacked This Frame` true)
        (`GameplayStatics.PlaySound2D` (`self.Attack Sound`) 1.0 1.0 0.0 null null)
        (else
          ;[1 1 1] Check if we finished the attacking animation
          (if (and (`|EnumEquality` (`self.Character State`) "NewEnumerator4") (not (`PaperFlipbookComponent.IsPlaying` (`self.Sprite`))))
            (`self.End Attack`)
            (set `self.Attacked This Frame` false)
            (set `self.Attack Interval Timer` 0.0)
            (else
              ;[1 1 1] Check if we reached jump apex
              (if (and (`|EnumEquality` "NewEnumerator2" (`self.Character State`)) (< _returnvalue_z_2 0.0))
                (`self.Peak Jump`)
                (else
                  ;[1 1 1] Check if we reached the ground when falling
                  (if (and (`|EnumEquality` "NewEnumerator3" (`self.Character State`)) (== 0.0 _returnvalue_z))
                    (`self.End Falling`)))))))))))

(fn `UserConstructionScript`
  (`parent.UserConstructionScript`)
  ;[1 1 1] Set Attack Interval timer so he can attack
  (set `self.Attack Interval Timer` (`self.Attack Interval`)))