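; Controller for an enemy pawn that chases and attacks the player along the horizontal X axis.
; Each Tick, unless the player is dying, an unobstructed Visibility trace within the enemy's sight distance drives movement toward the player's side.
; Attacks are attempted at close range while chasing.
; A triggered flag makes losing sight end movement once, followed by a final attack range check.
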(event `self.ReceiveBeginPlay`
  (bind _asbp_enemy (cast `/Game/Blueprints/Characters/BP_Enemy` (`self.K2_GetPawn`))
    (:`then`
      (set `self.Enemy` _asbp_enemy))
    (:`CastFailed`
      _))
  (bind _asbp_player (cast `/Game/Blueprints/Characters/BP_Player` (`GameplayStatics.GetPlayerPawn` 0)))
  (set `self.Player` _asbp_player))

(event `self.ReceiveTick`
  (params (DeltaSeconds :type "Float (single-precision)"))
  ;[1 1 1] Check if player is dying
  (if (`|EnumInequality` "NewEnumerator5" (`/Game/Blueprints/Characters/BP_Character.Character State` (`self.Player`)))
    ;[1 1 1] Horizontal Movement
    (bind _in_line_of_sight (`self.In Line Of Sight`))
    (if _in_line_of_sight
      (bind _action_value (`self.Get Action Value`))
      (`/Game/Blueprints/Characters/BP_Character.Moving` (`self.Enemy`) _action_value)
      (set `self.Triggerd` true)
      ;[1 1 1] Attack
      (if (<= (`KismetMathLibrary.Vector_Distance2D` (`self.K2_GetActorLocation` (`self.Enemy`)) (`self.K2_GetActorLocation` (`self.Player`))) 25.0) :!label _label
        (`/Game/Blueprints/Characters/BP_Character.Try Attack` (`self.Enemy`)))
      (elif (`self.Triggerd`)
        (`/Game/Blueprints/Characters/BP_Character.End Moving` (`self.Enemy`))
        (set `self.Triggerd` false)
        (goto _label)))))

(fn `Get Action Value`
  (returns (`Action Value` :type "Float (double-precision)"))
  (bind _returnvalue_x (`KismetMathLibrary.BreakVector` (`self.K2_GetActorLocation` (`self.Player`))))
  (bind _returnvalue_x_2 (`KismetMathLibrary.BreakVector` (`self.K2_GetActorLocation` (`self.Enemy`))))
  (if (> _returnvalue_x _returnvalue_x_2)
    (return 1.0)
    (else
      (return -1.0))))

(fn `In Line Of Sight`
  (returns (`In Line Of Sight` :type Boolean))
  ;[1 1 1] Line trace to player if it hit someting then there is no line of sight on the player
  (bind (_outhit _returnvalue) (`KismetSystemLibrary.LineTraceSingle` (`self.K2_GetActorLocation` (`self.Enemy`)) (`self.K2_GetActorLocation` (`self.Player`)) "TraceTypeQuery1"))
  (if _returnvalue
    _
    (elif (<= (`KismetMathLibrary.VSize` (- (`.TraceEnd` (`GameplayStatics.BreakHitResult` _outhit)) (`.TraceStart` (`GameplayStatics.BreakHitResult` _outhit)))) (`/Game/Blueprints/Characters/BP_Enemy.Line Of Sight Distance` (`self.Enemy`)))
      (return true)
      (else
        _)))
  (return false))

(fn `UserConstructionScript`)